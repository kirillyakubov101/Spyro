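; Spyro character Blueprint that adds a one-use glide to jumping.
; The jump event calls Jump, then starts gliding if CanGlide is set and the character is airborne after a jump, clearing the flag; otherwise it stops gliding.
; Tick checks the movement component and, while on the ground, stops gliding and restores CanGlide.
; A separate event stops jumping without ending the glide.
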(event EventTick
  (params (DeltaSeconds :type Float%20%28single-precision%29))
  (if (AI|Components|NavMovement|IsMovingonGround (Variables|Character|GetCharacterMovement))
    (Class|SpyroCharacter|StopGliding)
    (Variables|Default|SetCanGlide true)))

(event EventStopJumpEvent
  (Character|StopJumping))

(event EventJumpEvent
  (Character|Jump)
  (if (and (Variables|Default|GetCanGlide) (Class|SpyroCharacter|IsAirbornAfterJump))
    (Class|SpyroCharacter|Glide)
    (Variables|Default|SetCanGlide false)
    (else
      (Class|SpyroCharacter|StopGliding))))

(fn ConstructionScript)